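; BP_Car is a drivable physics vehicle, a Box body with a Paper2D flipbook sprite, driven through Enhanced Input.
; Each tick, four wheel line traces apply compression-scaled suspension forces, and each grounded wheel adds forward force from the smoothed AccelerationInput.
; That input eases back toward zero, and steering applies yaw torque scaled by it.
; Raw A and D key events separately swap the turn and drive flipbooks.
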(event `self.ReceiveBeginPlay`
  (`EnhancedInputSubsystemInterface.AddMappingContext` (pcsubsystem `EnhancedInputLocalPlayerSubsystem` (`GameplayStatics.GetPlayerController` 0)) "/Game/Vehicles/Inputs/IMC_Vehicle.IMC_Vehicle" 0 (struct)))

(event `EnhancedInput|/Game/Vehicles/Inputs/IA_Accelerate`
  (params (ActionValue :type "Float (double-precision)") (ElapsedSeconds :type "Float (double-precision)") (TriggeredSeconds :type "Float (double-precision)") (InputAction :type "InputAction Object Reference" :default "/Game/Vehicles/Inputs/IA_Accelerate.IA_Accelerate"))
  (:`Triggered`
    (set `self.AccelerationInput` (`KismetMathLibrary.FInterpTo` (`self.AccelerationInput`) ActionValue (`GameplayStatics.GetWorldDeltaSeconds`) 0.5))))

(event `Key|A`
  (params (Key :type "Key Structure"))
  (bind _paperflipbook (`self.PaperFlipbook`))
  (:`Pressed`
    (set `self.A Pressed` true)
    (`PaperFlipbookComponent.PlayFromStart` (`self.PaperFlipbook`))
    (`KismetSystemLibrary.DelayUntilNextTick`)
    ;[1 1 1] Set Left turn sprite
    (`PaperFlipbookComponent.SetFlipbook` (`self.PaperFlipbook`) "/Game/Vehicles/Car/FB_Car_turn_left.FB_Car_turn_left")
    (if (`PaperFlipbookComponent.IsPlaying` (`self.PaperFlipbook`))
      (`PaperFlipbookComponent.SetLooping` (`self.PaperFlipbook`) false)
      (else
        (`PaperFlipbookComponent.SetLooping` (`self.PaperFlipbook`) true))))
  (:`Released`
    (bind _output_get (set `self.A Pressed` false))
    (if (`KismetMathLibrary.BooleanNOR` _output_get (stale `Key|D` _output_get)) :!label _label
      ;[1 1 1] reset Sprite
      (`PaperFlipbookComponent.SetLooping` _paperflipbook true)
      (`PaperFlipbookComponent.Play` _paperflipbook)
      (`PaperFlipbookComponent.SetFlipbook` (`self.PaperFlipbook`) "/Game/Vehicles/Car/Flipbooks/FB_Car_Drive.FB_Car_Drive"))))

(event `self.ReceiveTick`
  (params (DeltaSeconds :type "Float (single-precision)"))
  ;[1 1 1] Wheels location relative to ground/ suspension code
  (`self.SuspensionCast` (`self.FL_Wheel`))
  (`self.SuspensionCast` (`self.FR_Wheel`))
  (`self.SuspensionCast` (`self.BL_Wheel`))
  (`self.SuspensionCast` (`self.BR_Wheel`))
  (`self.CalculateAcceleration`))

(event `EnhancedInput|/Game/Vehicles/Inputs/IA_Steer`
  (params (ActionValue :type "Float (double-precision)") (ElapsedSeconds :type "Float (double-precision)") (TriggeredSeconds :type "Float (double-precision)") (InputAction :type "InputAction Object Reference" :default "/Game/Vehicles/Inputs/IA_Steer.IA_Steer"))
  (:`Triggered`
    (`PrimitiveComponent.AddTorqueInRadians` (`self.Box`) (`KismetMathLibrary.MakeVector` 0.0 0.0 (* ActionValue 1000000.0 (`self.AccelerationInput`))) "None" false)))

(event `Key|D`
  (params (Key :type "Key Structure"))
  (:`Pressed`
    (set `self.D Pressed` true)
    (`PaperFlipbookComponent.PlayFromStart` (`self.PaperFlipbook`))
    (`KismetSystemLibrary.DelayUntilNextTick`)
    ;[1 1 1] set right turn sprite
    (`PaperFlipbookComponent.SetFlipbook` (`self.PaperFlipbook`) "/Game/Vehicles/Car/FB_Car_Turn_Right.FB_Car_Turn_Right")
    (if (`PaperFlipbookComponent.IsPlaying` (`self.PaperFlipbook`))
      (`PaperFlipbookComponent.SetLooping` (`self.PaperFlipbook`) false)
      (else
        (`PaperFlipbookComponent.SetLooping` (`self.PaperFlipbook`) true))))
  (:`Released`
    (bind _output_get (set `self.D Pressed` false))
    (goto _label)))

(event `EnhancedInput|/Game/Vehicles/Inputs/IA_Steer`
  (params (ActionValue :type "Float (double-precision)") (ElapsedSeconds :type "Float (double-precision)") (TriggeredSeconds :type "Float (double-precision)") (InputAction :type "InputAction Object Reference" :default "/Game/Vehicles/Inputs/IA_Steer.IA_Steer")))

(fn `AccelerateCar`
  (params (WheelComp :type "SceneComponent Object Reference"))
  (bind _box (`self.Box`))
  (`PrimitiveComponent.AddForceAtLocation` (`self.Box`) (* (`SceneComponent.GetForwardVector` _box) 4000.0 (`self.AccelerationInput`) (`PrimitiveComponent.GetMass` _box)) (`SceneComponent.K2_GetComponentLocation` WheelComp) "None"))

(fn `CalculateAcceleration`
  (bind _accelerationinput (`self.AccelerationInput`))
  (set `self.Acceleration` (* (`KismetMathLibrary.Lerp` 0.0 2500.0 _accelerationinput) _accelerationinput))
  (set `self.AccelerationInput` (`KismetMathLibrary.FInterpTo` (`self.AccelerationInput`) 0.0 (`GameplayStatics.GetWorldDeltaSeconds`) 0.3)))

(fn `SuspensionCast`
  (params (WheelComp :type "SceneComponent Object Reference"))
  (bind _returnvalue (`SceneComponent.K2_GetComponentLocation` WheelComp))
  (bind _outhit (`KismetSystemLibrary.LineTraceSingle` :`Start` _returnvalue :`End` (+ _returnvalue (* (`SceneComponent.GetUpVector` WheelComp) -60.0)) :`TraceChannel` "TraceTypeQuery1" :`DrawDebugType` "ForOneFrame"))
  (bind (_bblockinghit _binitialoverlap _time _distance _location _impactpoint _normal _impactnormal _physmat _hitactor _hitcomponent _hitbonename _bonename _hititem _elementindex _faceindex _tracestart _traceend) (`GameplayStatics.BreakHitResult` _outhit))
  (if _bblockinghit
    (`PrimitiveComponent.AddForceAtLocation` (`self.Box`) (* (- 1.0 (`KismetMathLibrary.NormalizeToRange` _distance 0.0 60.0)) (`KismetMathLibrary.GetDirectionUnitVector` _traceend _tracestart) 90000.0) (`SceneComponent.K2_GetComponentLocation` (`local.WheelComp`)) "None")
    (`self.AccelerateCar` (`local.WheelComp`))))

(fn `UserConstructionScript`)