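; GM_car, apparently the car game mode, keeps an elapsed minutes-and-seconds timer and puts the WBP_Timer widget on screen at BeginPlay.
; While TimerRunning is true, Tick feeds a one-second Delay that increments Seconds and rolls it over into Minutes.
; The count relies on Delay ignoring repeat triggers, so it is only approximately one second per step.
; Nothing here sets TimerRunning or passes the time to the widget.
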(event `self.ReceiveBeginPlay`
  (bind _returnvalue (`|CreateWidget` "/Game/WBP_Timer.WBP_Timer_C"))
  (`UserWidget.AddToViewport` _returnvalue 0))

(event `self.ReceiveTick`
  (params (DeltaSeconds :type "Float (single-precision)"))
  (if (`self.TimerRunning`)
    (`KismetSystemLibrary.Delay` 1.0)
    (set `self.Seconds` (+ (`self.Seconds`) 1))
    (if (> (`self.Seconds`) 59)
      (set `self.Minutes` (+ (`self.Minutes`) 1))
      (set `self.Seconds` 0))))

(fn `UserConstructionScript`)