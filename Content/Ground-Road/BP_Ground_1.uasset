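; BP_Ground_1 is a self-replicating road segment that keeps ground generating ahead of the player's BP_Car.
; When the car enters CreateBox, it spawns another BP_Ground_1 at the Arrow component's transform.
; When the car enters DeleteBox, the segment destroys itself.
; The car reference is cached from player pawn 0 on BeginPlay, and both triggers print debug messages.
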(event `self.ReceiveBeginPlay`
  (bind _asbp_car (cast `/Game/Vehicles/BP_Car` (`GameplayStatics.GetPlayerPawn` 0)))
  (set `self.As BP Car` _asbp_car))

(event `self.CreateBox.OnComponentBeginOverlap`
  (params (OverlappedComponent :type "PrimitiveComponent Object Reference") (OtherActor :type "Actor Object Reference") (OtherComp :type "PrimitiveComponent Object Reference") (OtherBodyIndex :type Integer) (bFromSweep :type Boolean) (SweepResult :type "HitResult Structure (by ref)"))
  ;[0.4609 0.4609 0.4609] Create Ground
  (if (== OtherActor (`self.As BP Car`))
    (`|SpawnActorFromClass` "BP_Ground_1_C" (`SceneComponent.K2_GetComponentToWorld` (`self.Arrow`)) "Undefined" "MultiplyWithRoot" null (`GameplayStatics.GetPlayerCharacter` 0))
    (`KismetSystemLibrary.PrintString` "SPAWNED")))

(event `self.DeleteBox.OnComponentBeginOverlap`
  (params (OverlappedComponent :type "PrimitiveComponent Object Reference") (OtherActor :type "Actor Object Reference") (OtherComp :type "PrimitiveComponent Object Reference") (OtherBodyIndex :type Integer) (bFromSweep :type Boolean) (SweepResult :type "HitResult Structure (by ref)"))
  ;[0.2682 0.2682 0.2682] Delete Ground
  (if (== OtherActor (`self.As BP Car`))
    (`self.K2_DestroyActor`)
    (`KismetSystemLibrary.PrintString` "DELETED")))

(fn `UserConstructionScript`)