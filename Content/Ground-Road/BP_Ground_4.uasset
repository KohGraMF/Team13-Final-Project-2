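; BP_Ground_4 is a road ground segment that spawns the next segment and removes itself in response to the car.
; When AsBPCar overlaps CreateBox, it spawns BP_Ground_5 at the Arrow component's world transform, chaining the road forward.
; When AsBPCar overlaps DeleteBox, the segment destroys itself.
; Both events print debug strings, and nothing in this file assigns the AsBPCar reference they compare against.
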(event `self.CreateBox.OnComponentBeginOverlap`
  (params (OverlappedComponent :type "PrimitiveComponent Object Reference") (OtherActor :type "Actor Object Reference") (OtherComp :type "PrimitiveComponent Object Reference") (OtherBodyIndex :type Integer) (bFromSweep :type Boolean) (SweepResult :type "HitResult Structure (by ref)"))
  ;[0.4609 0.4609 0.4609] Create Ground
  (if (== OtherActor (`self.As BP Car`))
    (`|SpawnActorFromClass` "/Game/Ground-Road/BP_Ground_5.BP_Ground_5_C" (`SceneComponent.K2_GetComponentToWorld` (`self.Arrow`)) "Undefined" "MultiplyWithRoot" null (`GameplayStatics.GetPlayerCharacter` 0))
    (`KismetSystemLibrary.PrintString` "SPAWNED")))

(event `self.DeleteBox.OnComponentBeginOverlap`
  (params (OverlappedComponent :type "PrimitiveComponent Object Reference") (OtherActor :type "Actor Object Reference") (OtherComp :type "PrimitiveComponent Object Reference") (OtherBodyIndex :type Integer) (bFromSweep :type Boolean) (SweepResult :type "HitResult Structure (by ref)"))
  ;[0.2682 0.2682 0.2682] Delete Ground
  (if (== OtherActor (`self.As BP Car`))
    (`self.K2_DestroyActor`)
    (`KismetSystemLibrary.PrintString` "DELETED")))

(fn `UserConstructionScript`
  (`parent.UserConstructionScript`))